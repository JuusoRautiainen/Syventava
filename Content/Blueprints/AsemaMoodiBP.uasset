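; Game mode Blueprint that respawns the player whenever their pawn is destroyed.
; BeginPlay binds Tuhoutunut to player pawn 0's OnDestroyed event, and the Respawn event repeats that binding for each new pawn.
; RespawnPlayer spawns the default pawn class at the "aloitus" player start and has player controller 0 possess it.
; Tuhoutunut calls RespawnPlayer twice in succession before rebinding, so each death spawns two pawns.
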(event Custom|Tuhoutunut
  (params (DestroyedActor :type Actor%20Object%20Reference))
  (CallFunction|RespawnPlayer)
  (CallFunction|RespawnPlayer)
  (CallFunction|Respawn))

(event Custom|Respawn
  (Game|BindEventtoOnDestroyed (Game|Player|GetPlayerPawn 0) (delegate Custom|Tuhoutunut)))

(event EventBeginPlay
  (Game|BindEventtoOnDestroyed (Game|Player|GetPlayerPawn 0) (delegate Custom|Tuhoutunut)))

(event EventTick
  (params (DeltaSeconds :type Float%20%28single-precision%29)))

(fn ConstructionScript)

(fn RespawnPlayer
  (bind _returnvalue (Game|SpawnActorfromClass (Variables|Default|GetDefaultPawnClass) (Transformation|GetActorTransform (Class|GameModeBase|FindPlayerStart 0 "aloitus")) "Undefined" 0 0))
  (Pawn|Possess (Game|GetPlayerController 0) _returnvalue))